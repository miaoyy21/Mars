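; BP_Tilemap is a tilemap actor whose side triggers pause a player's camera at the left and right edges.
; Begin and end overlaps on LeftSide and RightSide feed a shared OnOverlapSide event with a paused flag set on entry and cleared on exit.
; That event acts only with authority, filters for actors tagged Player, and passes the flag to PausePlayerCamera through the object returned by GetPlayerMessage.
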(event OnComponentBeginOverlap(LeftSide)
  (params (OverlappedComponent :type Primitive%20Component%20Object%20Reference) (OtherActor :type Actor%20Object%20Reference) (OtherComp :type Primitive%20Component%20Object%20Reference) (OtherBodyIndex :type Integer) (bFromSweep :type Boolean) (SweepResult :type Hit%20Result%20Structure%20%28by%20ref%29))
  (CallFunction|OnOverlapSide OtherActor true))

(event OnComponentEndOverlap(LeftSide)
  (params (OverlappedComponent :type Primitive%20Component%20Object%20Reference) (OtherActor :type Actor%20Object%20Reference) (OtherComp :type Primitive%20Component%20Object%20Reference) (OtherBodyIndex :type Integer))
  (CallFunction|OnOverlapSide OtherActor false))

(event OnComponentBeginOverlap(RightSide)
  (params (OverlappedComponent :type Primitive%20Component%20Object%20Reference) (OtherActor :type Actor%20Object%20Reference) (OtherComp :type Primitive%20Component%20Object%20Reference) (OtherBodyIndex :type Integer) (bFromSweep :type Boolean) (SweepResult :type Hit%20Result%20Structure%20%28by%20ref%29))
  (CallFunction|OnOverlapSide OtherActor true))

(event OnComponentEndOverlap(RightSide)
  (params (OverlappedComponent :type Primitive%20Component%20Object%20Reference) (OtherActor :type Actor%20Object%20Reference) (OtherComp :type Primitive%20Component%20Object%20Reference) (OtherBodyIndex :type Integer))
  (CallFunction|OnOverlapSide OtherActor false))

(event Custom|OnOverlapSide
  (params (目标 :type Actor%20Object%20Reference) (Paused :type Boolean))
  (Networking|SwitchHasAuthority
    (:Authority
      (if (Actor|ActorHasTag 目标 "Player")
        (bind _player (Class|INFPlayer|GetPlayer(Message) 目标))
        (Default|PausePlayerCamera _player Paused)))))

(fn ConstructionScript)