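; BP_Climbing is a climbable actor whose box volume marks where players can climb.
; Box begin and end overlaps feed a shared SetClimbing event, which acts only with authority and only on actors tagged Player.
; It passes the climb state to the player's message object via SetClimbingMessage, including itself as the climbing actor when climbing becomes available.
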(event OnComponentBeginOverlap(Box)
  (params (OverlappedComponent :type Primitive%20Component%20Object%20Reference) (OtherActor :type Actor%20Object%20Reference) (OtherComp :type Primitive%20Component%20Object%20Reference) (OtherBodyIndex :type Integer) (bFromSweep :type Boolean) (SweepResult :type Hit%20Result%20Structure%20%28by%20ref%29))
  (CallFunction|SetClimbing OtherActor true))

(event OnComponentEndOverlap(Box)
  (params (OverlappedComponent :type Primitive%20Component%20Object%20Reference) (OtherActor :type Actor%20Object%20Reference) (OtherComp :type Primitive%20Component%20Object%20Reference) (OtherBodyIndex :type Integer))
  (CallFunction|SetClimbing OtherActor false))

(event Custom|SetClimbing
  (params (Actor :type Actor%20Object%20Reference) (CanClimbing :type Boolean))
  ;[1 1 1] 设置玩家的攀爬状态
  (Networking|SwitchHasAuthority
    (:Authority
      (if (Actor|ActorHasTag Actor "Player")
        (bind _player (Class|INFPlayer|GetPlayer(Message) Actor))
        (if CanClimbing
          (Class|INFPlayer|SetClimbing(Message) _player true self)
          (else
            (Class|INFPlayer|SetClimbing(Message) _player false)))))))

(fn ConstructionScript)