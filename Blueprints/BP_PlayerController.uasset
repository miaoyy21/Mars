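; Player controller that handles player selection and spawning.
; On BeginPlay, a client event creates and displays the WB_PlayerSelection widget.
; A selected player class and location pass through a server event to the GameMode's message interface as a spawn request.
; SpawnPlayer spawns the class at a given transform and possesses the pawn obtained through the spawned actor's GetPlayerMessage.
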(event Custom|CL_Initialize
  (bind _returnvalue (UserInterface|CreateWidget "/Game/Mars/Blueprints/UI/WB_PlayerSelection.WB_PlayerSelection_C"))
  (bind _output_get (Variables|Default|SetWB_PlayerSelection _returnvalue))
  (UserInterface|Viewport|AddtoViewport _output_get 0))

(event Custom|SRV_PlayerSelection
  (params (Player :type Actor%20Class%20Reference) (Location :type Vector))
  (bind _gamemode (Class|INFGameMode|GetGameMode(Message) (Game|GetGameMode)))
  (Class|INFGameMode|RequestSpawnPlayer(Message) _gamemode self Player Location))

(event EventBeginPlay
  (CallFunction|Initialize))

(event EventInitialize
  (CallFunction|CLInitialize))

(event EventPlayerSelection
  (params (Player :type Actor%20Class%20Reference) (Location :type Vector :default "0, 0, 0"))
  (CallFunction|SRVPlayerSelection Player Location))

(event EventSpawnPlayer
  (params (Player :type Actor%20Class%20Reference) (Transform :type Transform))
  (bind _returnvalue (Game|SpawnActorfromClass Player Transform "Undefined" "MultiplyWithRoot" 0 0))
  (bind _player (Class|INFPlayer|GetPlayer(Message) _returnvalue))
  (Pawn|Possess _player))

(fn ConstructionScript)

(fn GetPlayerController
  (return self))